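; Warrior character Blueprint that performs a sword melee attack through the Gameplay Ability System.
; On BeginPlay it acquires GA_MeleeAttack and attaches a spawned Sword to the right-hand socket.
; MainAttack activates the ability, then DoHitTrace box-overlaps Pawns ahead and sends itself a Skill.melee.dealDamage event with each as target.
; The debug box drawn is deeper than the actual overlap box, and the direct montage call is unconnected.
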(event EventBeginPlay
  (Class|CubeHero|AquireAbility "/Game/Blueprints/Abilities/GameplayAbilities/Warrior/GA_MeleeAttack.GA_MeleeAttack_C")
  (bind _returnvalue (Game|SpawnActorfromClass "/Game/Blueprints/Testing/Items/Sword.Sword_C" (Math|Transform|MakeTransform "0, 0, 0") "Undefined" 0 0))
  (Transformation|AttachComponentToComponent _returnvalue (Variables|Character|GetMesh) "RightHandWeapon" "SnapToTarget" "SnapToTarget" "SnapToTarget" true))

(event Collision|EventActorBeginOverlap
  (params (OtherActor :type Actor%20Object%20Reference)))

(event EventTick
  (params (DeltaSeconds :type Float%20%28single-precision%29)))

(event EventMainAttack
  (Abilities|TryActivateAbilitybyClass (Variables|Default|GetAbilitySystem) "/Game/Blueprints/Abilities/GameplayAbilities/Warrior/GA_MeleeAttack.GA_MeleeAttack_C" true)
  (CallFunction|DoHitTrace))

(fn ConstructionScript)

(fn DoHitTrace
  (bind _returnvalue (Transformation|GetActorLocation))
  (bind _capsulecomponent (Variables|Default|GetCapsuleComponent))
  (bind _returnvalue_2 (Math|Vector|GetForwardVector _capsulecomponent))
  (bind _returnvalue_3 (* _returnvalue_2 1e+02))
  (bind _returnvalue_4 (+ _returnvalue _returnvalue_3))
  (bind (_outactors _returnvalue_5) (Collision|BoxOverlapActors _returnvalue_4 "6.060000,50.000000,50.000000" (Utilities|Array|MakeArray "ObjectTypeQuery3") 0 (Utilities|Array|MakeArray self) :!class /Script/Engine.KismetSystemLibrary))
  (if _returnvalue_5
    (for _array_element _outactors
      (Ability|SendGameplayEventtoActor self "(TagName=\"skill.melee.dealDamage\")" (Utilities|Struct|MakeGameplayEventData "" 0 _array_element)))
    (Rendering|Debug|DrawDebugBox :Center _returnvalue_4 :Extent "60.000000,50.000000,50.000000" :Rotation (Transformation|GetActorRotation) :Duration 2.0 :Thickness 2.0)
    (Ability|SendGameplayEventtoActor self "(TagName=\"skill.melee.dealDamage\")" (Utilities|Struct|MakeGameplayEventData "" 0 _array_element))))